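; Interactable door that the first-person player cycles through closed, partially open and open, with a sound for each step.
; Tick polls the character's interaction flag and hit actor, sets the swing side by dot product, then interpolates yaw while interaction continues.
; A timer based on sound length variable DoorSoundTime advances the state.
; Optional auto-close fires after the player exits the box facing roughly along world Y, using one interpolation step.
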(event `self.ReceiveBeginPlay`
  (bind _asbp_first_person_character (cast `/Game/FirstPerson/Blueprints/BP_FirstPersonCharacter` (`GameplayStatics.GetPlayerCharacter` 0)))
  (set `self.Character Ref` _asbp_first_person_character))

(event `self.ReceiveTick`
  (params (DeltaSeconds :type "Float (single-precision)"))
  (bind _character_ref (`self.Character Ref`))
  (if (and (`/Game/FirstPerson/Blueprints/BP_FirstPersonCharacter.is Interacting?` _character_ref) (== (`/Game/FirstPerson/Blueprints/BP_FirstPersonCharacter.Hit Actor` _character_ref) self))
    (if (`self.bIsInteractingWithDoor?`)
      (`self.HandleDoor`)
      (else
        (`self.isInteractingWithDoor` (`self.Character Ref`))))))

(event `self.Box Collision.OnComponentEndOverlap`
  (params (OverlappedComponent :type "PrimitiveComponent Object Reference") (OtherActor :type "Actor Object Reference") (OtherComp :type "PrimitiveComponent Object Reference") (OtherBodyIndex :type Integer))
  (bind _returnvalue (`GameplayStatics.GetPlayerCharacter` 0))
  (bind (_returnvalue_x _returnvalue_y) (`KismetMathLibrary.BreakVector` (`self.GetActorForwardVector` _returnvalue)))
  ;[0.4375 0.291 0] Automatic Door Closed
  (if (and (`self.autoClose?`) (`self.doorOpen?`))
    (if (and (== OtherActor _returnvalue) (or (>= _returnvalue_y 0.7) (<= _returnvalue_y -0.7)))
      (`KismetSystemLibrary.Delay` 0.5)
      (`self.AutoClose Door`)
      (set `self.autoCloseActivated?` true))))

(event `isInteractingWithDoor`
  (params (Player :type "/Game/FirstPerson/Blueprints/BP_FirstPersonCharacter Object Reference"))
  ;[0.4375 0.291 0] Door Interaction Math
  (if (`self.autoCloseActivated?`)
    (set `self.EDoorStates` "NewEnumerator0")
    (set `self.autoCloseActivated?` false))
  (`self.Door StateSounds`)
  (if (> (`KismetMathLibrary.Dot_VectorVector` (`self.GetActorForwardVector` Player) (`SceneComponent.GetForwardVector` (`self.DoorOpenLocation`))) 0.0)
    (set `self.Door Open Side` 1.0)
    (else
      (set `self.Door Open Side` -1.0)))
  (set `self.bIsInteractingWithDoor?` true)
  (`KismetSystemLibrary.K2_SetTimerDelegate` (delegate `CustomEvent`) (`self.Door Sound Time`)))

(event `AutoClose Door`
  ;[0.4375 0.291 0] Automatic Door Closed
  ;;[0.4375 0.291 0] Closing Door Function
  (`GameplayStatics.PlaySoundAtLocation` "/Game/Door/Audio/closeddoor.closeddoor" (`self.K2_GetActorLocation`) (struct) 1.0 1.0 0.0 null null null null)
  (`SceneComponent.K2_SetRelativeRotation` (`self.Door`) (`KismetMathLibrary.MakeRotator` 0.0 0.0 (`KismetMathLibrary.FInterpTo` (.yaw (`SceneComponent.RelativeRotation` (`self.Door`))) 0.0 5.0 (`self.Interp Speed`))) false false))

(event `CustomEvent`
  ;[0.4375 0.291 0] Door Interaction Math
  (set `self.bIsInteractingWithDoor?` false)
  (switch `/Game/Door/E_DoorStates` (`self.EDoorStates`)
    (:`NewEnumerator0`
      (set `self.EDoorStates` "NewEnumerator1"))
    (:`NewEnumerator1`
      (set `self.EDoorStates` "NewEnumerator2"))
    (:`NewEnumerator2`
      (set `self.EDoorStates` "NewEnumerator0"))))

(event `Door StateSounds`
  (bind _returnvalue (`self.K2_GetActorLocation`))
  ;[0.6719 0.4242 0.02239] Door SFX
  (switch `/Game/Door/E_DoorStates` (`self.EDoorStates`)
    (:`NewEnumerator0`
      (`GameplayStatics.PlaySoundAtLocation` "/Game/Door/Audio/partially.partially" _returnvalue (struct) 1.0 1.0 0.0 null null null null))
    (:`NewEnumerator1`
      (`GameplayStatics.PlaySoundAtLocation` "/Game/Door/Audio/opendoor.opendoor" _returnvalue (struct) 1.0 1.0 0.0 null null null null))
    (:`NewEnumerator2`
      (`GameplayStatics.PlaySoundAtLocation` "/Game/Door/Audio/closeddoor.closeddoor" _returnvalue (struct) 1.0 1.0 0.0 null null null null))))

(event `HandleDoor`
  ;[0.6719 0.4242 0.02239] Handle Door (Rotasi Pintu tergantung dari Door Statenya)
  (switch `/Game/Door/E_DoorStates` (`self.EDoorStates`)
    (:`NewEnumerator0`
      (`self.HandleRotation` (* 15.0 (`self.Door Open Side`)))
      (set `self.doorOpen?` true))
    (:`NewEnumerator1`
      (`self.HandleRotation` (* (`self.Door Open Angle`) (`self.Door Open Side`)))
      (set `self.doorOpen?` true))
    (:`NewEnumerator2`
      (if (== (`self.Door Open Side`) 1.0)
        (`self.HandleRotation` -5.0)
        (else
          (`self.HandleRotation` 5.0)))
      (set `self.doorOpen?` false))))

(event `HandleRotation`
  (params (`Set Rotation` :type "Float (double-precision)"))
  ;[0.5104 0.3023 0] Handle Rotation
  (`SceneComponent.K2_SetRelativeRotation` (`self.Door`) (`KismetMathLibrary.MakeRotator` 0.0 0.0 (`KismetMathLibrary.FInterpTo` (.yaw (`SceneComponent.RelativeRotation` (`self.Door`))) `Set Rotation` (`GameplayStatics.GetWorldDeltaSeconds`) (`self.Interp Speed`))) false false))

(fn `Interact`
  (params (Interactor :type "Character Object Reference"))
  (returns (`did Interact?` :type Boolean))
  (return false))

(fn `UserConstructionScript`)