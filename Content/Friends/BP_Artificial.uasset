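; BP_Artificial is an NPC that can patrol and talk, then give way to a boss.
; In one State, it loops through Destinations using AI MoveTo.
; Each Talk call halts walking and advances a WBP_Dialogue widget; after the last line it removes the widget, spawns BP_realBoss at SpawnBossRef if valid, and destroys itself.
; Inner and outer overlap spheres swap interact icons by player proximity.
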(event `self.ReceiveBeginPlay`
  (bind _returnvalue (+ (`self.Target`) 1))
  ;[0.03646 0.03646 0.03646] Start
  (if (`|EnumEquality` (`self.State`) "NewEnumerator1")
    (`|AIMoveTo` self (0.0 0.0 0.0) (`|GetArrayItem` (`self.Destinations`) (`self.Target`)) :!label _label
      (:`OnSuccess`
        (if (== _returnvalue (`KismetArrayLibrary.Array_Length` (`self.Destinations`)))
          (set `self.Target` 0)
          (goto _label)
          (else
            (set `self.Target` _returnvalue)
            (goto _label)))))))

(event `/Game/Friends/BPI_Dialogue.Talk`
  (set `CharacterMovementComponent.MaxWalkSpeed` 0.0 (`self.CharacterMovement`))
  (`/Engine/EditorBlueprintResources/StandardMacros.IncrementInt` (`self.talkIndex`)
    (:`  `
      (if (< (`self.talkIndex`) (`KismetArrayLibrary.Array_Length` (`self.dialogue`)))
        (`self.UI`
          (:`then`
            _)
          (:`else`
            (bind _returnvalue (`|CreateWidget` "/Game/Friends/WBP_Dialogue.WBP_Dialogue_C" (`GameplayStatics.GetPlayerController` 0)))
            (bind _output_get (set `self.UI` _returnvalue))
            (`UserWidget.AddToViewport` _output_get 0)))
        (`TextBlock.SetText` (`/Game/Friends/WBP_Dialogue.TalkText` (`self.UI`)) (`KismetTextLibrary.Conv_StringToText` (`|GetArrayItem` (`self.dialogue`) (`self.talkIndex`))))
        (else
          (`Widget.RemoveFromParent` (`self.UI`))
          (`KismetSystemLibrary.Delay` 1.0)
          (`self.End Dialogue`)
          (`self.K2_DestroyActor`))))))

(event `End Dialogue`
  (bind _spawnboss_ref (`self.spawnBoss Ref`))
  (if (`KismetSystemLibrary.IsValid` _spawnboss_ref)
    (`|SpawnActorFromClass` "/Game/Enemy/Boss/AI/BP_realBoss.BP_realBoss_C" (`KismetMathLibrary.Conv_VectorToTransform` (`self.K2_GetActorLocation` _spawnboss_ref)) "Undefined" "MultiplyWithRoot" null null)))

(event `self.innerSphereCollision.OnComponentBeginOverlap`
  (params (OverlappedComponent :type "PrimitiveComponent Object Reference") (OtherActor :type "Actor Object Reference") (OtherComp :type "PrimitiveComponent Object Reference") (OtherBodyIndex :type Integer) (bFromSweep :type Boolean) (SweepResult :type "HitResult Structure (by ref)"))
  (if (== OtherActor (`GameplayStatics.GetPlayerCharacter` 0))
    (`SceneComponent.SetVisibility` (`self.innerInteractIcon`) true false)
    (`SceneComponent.SetVisibility` (`self.outerInteractIcon`) false false)))

(event `self.innerSphereCollision.OnComponentEndOverlap`
  (params (OverlappedComponent :type "PrimitiveComponent Object Reference") (OtherActor :type "Actor Object Reference") (OtherComp :type "PrimitiveComponent Object Reference") (OtherBodyIndex :type Integer))
  (if (== (`GameplayStatics.GetPlayerCharacter` 0) OtherActor)
    (`SceneComponent.SetVisibility` (`self.innerInteractIcon`) false false)
    (`SceneComponent.SetVisibility` (`self.outerInteractIcon`) true false)))

(event `self.outerSphereCollision.OnComponentBeginOverlap`
  (params (OverlappedComponent :type "PrimitiveComponent Object Reference") (OtherActor :type "Actor Object Reference") (OtherComp :type "PrimitiveComponent Object Reference") (OtherBodyIndex :type Integer) (bFromSweep :type Boolean) (SweepResult :type "HitResult Structure (by ref)"))
  (if (== OtherActor (`GameplayStatics.GetPlayerCharacter` 0))
    (`SceneComponent.SetVisibility` (`self.outerInteractIcon`) true false)))

(event `self.outerSphereCollision.OnComponentEndOverlap`
  (params (OverlappedComponent :type "PrimitiveComponent Object Reference") (OtherActor :type "Actor Object Reference") (OtherComp :type "PrimitiveComponent Object Reference") (OtherBodyIndex :type Integer))
  (if (== (`GameplayStatics.GetPlayerCharacter` 0) OtherActor)
    (`SceneComponent.SetVisibility` (`self.outerInteractIcon`) false false)))

(fn `UserConstructionScript`)