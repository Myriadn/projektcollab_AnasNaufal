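; Boss enemy character test with melee attacks, an HP bar and ragdoll death.
; BPCStats receives incoming damage and drives the widget's health bar, while three functions play attack montages.
; Begin/EndWeaponTrace toggle a looping timer that sphere-traces between weapon points, using a delayed DoOnce reset to throttle damage.
; PointDamageTrace adds a single-point damage sphere with camera shake, and Die disables movement, enables mesh physics and stops weapon traces from hitting.
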(event `self.ReceiveBeginPlay`
  ;[0.03646 0.03646 0.03646] begin play
  (bind _aswb_enemy_hp (cast `/Game/UI/WB_EnemyHP` (`WidgetComponent.GetWidget` (`self.Widget`))))
  (`/Game/FirstPerson/Blueprints/BPC_Stats.Set Player HP Progress Bar` (`self.BPC_Stats`) (`/Game/UI/WB_EnemyHP.HealthBar` _aswb_enemy_hp)))

(event `self.ReceiveAnyDamage`
  (params (Damage :type "Float (single-precision)") (DamageType :type "DamageType Object Reference") (InstigatedBy :type "Controller Object Reference") (DamageCauser :type "Actor Object Reference"))
  ;[0.03646 0.03646 0.03646] anyDamage
  (`/Game/FirstPerson/Blueprints/BPC_Stats.Increase Value` (`self.BPC_Stats`) "NewEnumerator0" (* Damage -1.0)))

(event `/Game/FirstPerson/Blueprints/BPI_Damage.End Weapon Trace`
  ;[0.03646 0.03646 0.03646] Traces
  (if (`KismetSystemLibrary.K2_IsValidTimerHandle` (stale `/Game/FirstPerson/Blueprints/BPI_Damage.Begin Weapon Trace` _returnvalue))
    (`KismetSystemLibrary.K2_ClearAndInvalidateTimerHandle` (stale `/Game/FirstPerson/Blueprints/BPI_Damage.Begin Weapon Trace` _returnvalue))))

(event `/Game/FirstPerson/Blueprints/BPI_Damage.Begin Weapon Trace`
  ;[0.03646 0.03646 0.03646] Traces
  (bind _returnvalue (`KismetSystemLibrary.K2_SetTimerDelegate` (delegate `Damage Trace`) 0.01 true)))

(event `Damage Trace`
  ;[0.03646 0.03646 0.03646] Traces
  (if (not (`self.isDead?`))
    (bind (_outhit _returnvalue) (`KismetSystemLibrary.SphereTraceSingleForObjects` :`Start` (`SceneComponent.K2_GetComponentLocation` (`self.Start Weapon Trace Pos`)) :`End` (`SceneComponent.K2_GetComponentLocation` (`self.End Weapon Trace Pos`)) :`Radius` (`self.swordAttackRadius`) :`ObjectTypes` (`|MakeArray` "ObjectTypeQuery3" :!type "EObjectTypeQuery Enum") :`DrawDebugType` "ForOneFrame"))
    (if _returnvalue
      (`/Engine/EditorBlueprintResources/StandardMacros.DoOnce` false :!label _label
        (:`Completed`
          (`GameplayStatics.ApplyDamage` (`.HitActor` (`GameplayStatics.BreakHitResult` _outhit)) (`self.weaponDamage`))
          (`KismetSystemLibrary.Delay` 0.3)
          (goto _label :!via `Reset`))))))

(event `/Game/FirstPerson/Blueprints/BPI_Damage.Die`
  ;[0.03646 0.03646 0.03646] Die
  (`CharacterMovementComponent.DisableMovement` (`self.CharacterMovement`))
  (`PrimitiveComponent.SetSimulatePhysics` (`self.Mesh`) true)
  (set `self.isDead?` true))

(event `/Game/FirstPerson/Blueprints/BPI_Damage.Point Damage Trace`
  (bind _returnvalue (`SceneComponent.K2_GetComponentLocation` (`self.Point Trace Pos`)))
  (`|ExecutionSequence`
    (:`then_0`
      (bind (_outhit _returnvalue_2) (`KismetSystemLibrary.SphereTraceSingleForObjects` :`Start` _returnvalue :`End` _returnvalue :`Radius` (`self.pointAttackRadius`) :`ObjectTypes` (`|MakeArray` "ObjectTypeQuery3" :!type "EObjectTypeQuery Enum") :`DrawDebugType` "ForDuration" :`DrawTime` 1.0))
      (if _returnvalue_2
        (`GameplayStatics.ApplyDamage` (`.HitActor` (`GameplayStatics.BreakHitResult` _outhit)) 10.0)))
    (:`then_1`
      (`GameplayStatics.PlayWorldCameraShake` "/Game/Enemy/Boss/AI/BP_CameraShake.BP_CameraShake_C" (`SceneComponent.K2_GetComponentLocation` (`self.Point Trace Pos`)) 0.0 2000.0))))

(fn `UserConstructionScript`)

(fn `Weapon Combo Attack`
  (returns (Duration :type "Float (double-precision)"))
  (bind _returnvalue (`self.PlayAnimMontage` (`self.weaponAttack`)))
  (return _returnvalue))

(fn `Weapon Heavy Attack`
  (returns (Duration :type "Float (double-precision)"))
  (bind _returnvalue (`self.PlayAnimMontage` (`self.heavyWeaponAttack`)))
  (return _returnvalue))

(fn `Weapon Slashing`
  (returns (Duration :type "Float (double-precision)"))
  (bind _returnvalue (`self.PlayAnimMontage` (`self.Anim Montage`)))
  (return _returnvalue))