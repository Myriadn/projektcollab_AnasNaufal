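; BP_AI is an enemy character that spots the player, performs a shove attack, and triggers the win screen when it takes any damage.
; PawnSensing sets the seeingPlayer blackboard key for Player-tagged pawns, while a looping timer periodically clears it.
; AttackPlayer plays a guarded montage and immediately sphere-traces forward from AttackTracePoint to apply damage.
; Any damage ragdolls the mesh, disables movement, shows WB_Win and plays victory sounds.
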(event `self.ReceiveBeginPlay`
  (`KismetSystemLibrary.K2_SetTimerDelegate` (delegate `Stop Seeing Player`) 0.8 true))

(event `Stop Seeing Player`
  (`BlackboardComponent.SetValueAsBool` (`AIBlueprintHelperLibrary.GetBlackboard` (`AIBlueprintHelperLibrary.GetAIController` self)) "seeingPlayer" false))

(event `self.PawnSensing.OnSeePawn`
  (params (Pawn :type "Pawn Object Reference"))
  (if (`self.ActorHasTag` Pawn "Player")
    (`BlackboardComponent.SetValueAsBool` (`AIBlueprintHelperLibrary.GetBlackboard` (`AIBlueprintHelperLibrary.GetAIController` self)) "seeingPlayer" true)))

(event `Attack Player`
  (bind _attack_trace_point (`self.Attack Trace Point`))
  (bind _returnvalue (`SceneComponent.K2_GetComponentLocation` _attack_trace_point))
  (if (not (`self.attacking?`))
    (set `self.attacking?` true)
    (`|PlayMontage` (`self.Mesh`) "/Game/AI/Paired_PushShove_Att_Montage.Paired_PushShove_Att_Montage"
      (:`then`
        (bind (_outhit _returnvalue_2) (`KismetSystemLibrary.SphereTraceSingleForObjects` _returnvalue (+ _returnvalue (* (`KismetMathLibrary.GetForwardVector` (`SceneComponent.K2_GetComponentRotation` _attack_trace_point)) 70.0)) 25.0 (`|MakeArray` "ObjectTypeQuery3" :!type "EObjectTypeQuery Enum")))
        (if _returnvalue_2
          (`GameplayStatics.ApplyDamage` (`.HitActor` (`GameplayStatics.BreakHitResult` _outhit)) 10.0)))
      (:`OnCompleted`
        (set `self.attacking?` false)))))

(event `self.ReceiveAnyDamage`
  (params (Damage :type "Float (single-precision)") (DamageType :type "DamageType Object Reference") (InstigatedBy :type "Controller Object Reference") (DamageCauser :type "Actor Object Reference"))
  (bind _returnvalue (`self.K2_GetActorLocation`))
  (`PrimitiveComponent.SetSimulatePhysics` (`self.Mesh`) true)
  (`CharacterMovementComponent.SetMovementMode` (`self.CharacterMovement`) "MOVE_None" 0)
  (bind _returnvalue_2 (`|CreateWidget` "/Game/FirstPerson/Widget/WB_Win.WB_Win_C"))
  (`UserWidget.AddToViewport` _returnvalue_2 0)
  (`GameplayStatics.PlaySoundAtLocation` "/Game/FirstPerson/Audio/Footsteps/victory.victory" _returnvalue (struct) 1.0 1.0 0.0 "/Game/FirstPerson/Audio/Footsteps/SA_Character.SA_Character" null null null)
  (`KismetSystemLibrary.Delay` 0.2)
  (`GameplayStatics.PlaySoundAtLocation` "/Game/FirstPerson/Audio/Footsteps/cinematic_boom.cinematic_boom" _returnvalue (struct) 1.0 1.0 0.0 null null null null))

(fn `UserConstructionScript`)